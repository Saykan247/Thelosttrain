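; BP_item is a collectible that the player picks up by pressing IA_PICKUP while near it.
; Overlap events on its Box enable input when the first-person character enters and disable it on exit.
; Pickup decrements Remaining on the first-person game mode, shows a WB_Collected widget and destroys the actor.
; An unconnected check for Remaining reaching zero is an empty placeholder for a victory response.
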(event `EnhancedInput|/Game/FirstPerson/Input/Actions/IA_PICKUP`
  (params (ActionValue :type Boolean) (ElapsedSeconds :type "Float (double-precision)") (TriggeredSeconds :type "Float (double-precision)") (InputAction :type "InputAction Object Reference" :default "/Game/FirstPerson/Input/Actions/IA_PICKUP.IA_PICKUP"))
  (:`Started`
    (bind _asbp_first_person_game_mode (cast `/Game/FirstPerson/Blueprints/BP_FirstPersonGameMode` (`GameplayStatics.GetGameMode`)))
    (bind _result (`/Engine/EditorBlueprintResources/StandardMacros.DecrementInt` (`/Game/FirstPerson/Blueprints/BP_FirstPersonGameMode.Remaining` _asbp_first_person_game_mode))
      (:`  `
        (set `/Game/FirstPerson/Blueprints/BP_FirstPersonGameMode.Remaining` _result _asbp_first_person_game_mode)
        (bind _returnvalue (`|CreateWidget` "/Game/Felipe/Items/WB_Collected.WB_Collected_C"))
        (`UserWidget.AddToViewport` _returnvalue 0)
        (`self.K2_DestroyActor`)))))

(event `self.Box.OnComponentBeginOverlap`
  (params (OverlappedComponent :type "PrimitiveComponent Object Reference") (OtherActor :type "Actor Object Reference") (OtherComp :type "PrimitiveComponent Object Reference") (OtherBodyIndex :type Integer) (bFromSweep :type Boolean) (SweepResult :type "HitResult Structure (by ref)"))
  (cast `/Game/FirstPerson/Blueprints/BP_FirstPersonCharacter` OtherActor)
  (`self.EnableInput` (`GameplayStatics.GetPlayerController` 0)))

(event `self.Box.OnComponentEndOverlap`
  (params (OverlappedComponent :type "PrimitiveComponent Object Reference") (OtherActor :type "Actor Object Reference") (OtherComp :type "PrimitiveComponent Object Reference") (OtherBodyIndex :type Integer))
  (cast `/Game/FirstPerson/Blueprints/BP_FirstPersonCharacter` OtherActor)
  (`self.DisableInput` (`GameplayStatics.GetPlayerController` 0)))

(fn `UserConstructionScript`)